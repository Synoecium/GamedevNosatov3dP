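; Player controller that owns the local player's UI: HUD, map selection, carousel switch menu and chat.
; On BeginPlay the local controller creates the widgets, keeping both menus hidden.
; Input actions toggle map selection and BP_HUD's chat window, and open the switch menu in UI-only mode, adjusting cursor and input mode.
; SwitchMenuClose restores game input, while AddWeapon forwards weapon icons to the carousel.
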(event Custom|SwitchMenuClose
  (Widget|SetVisibility (Variables|Default|GetWidgetSwitchMenu) "Hidden")
  (Input|SetInputModeGameOnly self)
  (Variables|Default|SetbShowMouseCursor false))

(event EventBeginPlay
  (if (Pawn|IsLocalController)
    (bind _returnvalue (UserInterface|CreateWidget "/Game/UI/WBP_HUD.WBP_HUD_C"))
    (UserInterface|Viewport|AddtoViewport _returnvalue 0)
    (bind _returnvalue_2 (UserInterface|CreateWidget "/Game/UI/WBP_MapSelectionWidget.WBP_MapSelectionWidget_C"))
    (bind _output_get (Variables|Default|SetWidgetMapSelection _returnvalue_2))
    (UserInterface|Viewport|AddtoViewport _returnvalue_2 0)
    (Widget|SetVisibility _output_get "Hidden")
    (bind _returnvalue_3 (UserInterface|CreateWidget "/Game/UI/WBP_CarouselClick.WBP_CarouselClick_C"))
    (bind _output_get_2 (Variables|Default|SetWidgetSwitchMenu _returnvalue_3))
    (UserInterface|Viewport|AddtoViewport _output_get_2 0)
    (Widget|SetVisibility _output_get_2 "Hidden")))

(event EventTick
  (params (DeltaSeconds :type Float%20%28single-precision%29)))

(event Input|ActionEvents|InputActionMapSelection
  (params (Key :type Key%20Structure :default "None"))
  (bind _self self)
  (bind _widgetmapselection (Variables|Default|GetWidgetMapSelection))
  (:Pressed
    (if (Widget|IsVisible _widgetmapselection)
      (Widget|SetVisibility _widgetmapselection "Hidden")
      (Input|SetInputModeGameOnly _self)
      (Variables|Default|SetbShowMouseCursor false)
      (else
        (Widget|SetVisibility _widgetmapselection "Visible")
        (Input|SetInputModeGameandUI _self (Variables|Default|GetWidgetMapSelection) "DoNotLock" true)
        (Variables|Default|SetbShowMouseCursor true)))))

(event Input|ActionEvents|InputActionSwitchMenu
  (params (Key :type Key%20Structure :default "None"))
  (:Pressed
    (Widget|SetVisibility (Variables|Default|GetWidgetSwitchMenu) "Visible")
    (Input|SetInputModeUIOnly self (Variables|Default|GetWidgetSwitchMenu) "LockAlways")
    (Variables|Default|SetbShowMouseCursor true)
    (Widget|SetKeyboardFocus (Variables|Default|GetWidgetSwitchMenu))))

(event Input|ActionEvents|InputActionChatMode
  (params (Key :type Key%20Structure :default "None"))
  (bind _self self)
  (:Pressed
    (bind _asbp_hud (Utilities|Casting|CastToBP_HUD (HUD|GetHUD)))
    (if (Pawn|IsLocalController)
      (if (Widget|IsVisible (Variables|/Script/GamedevNosatov3dP.MyHUD|GetChatWindow _asbp_hud))
        (Widget|SetVisibility (Variables|/Script/GamedevNosatov3dP.MyHUD|GetChatWindow _asbp_hud) "Hidden")
        (Input|SetInputModeGameOnly _self)
        (Variables|Default|SetbShowMouseCursor false)
        (else
          (Widget|SetVisibility (Variables|/Script/GamedevNosatov3dP.MyHUD|GetChatWindow _asbp_hud) "Visible")
          (Input|SetInputModeGameandUI _self 0 "DoNotLock" true)
          (Variables|Default|SetbShowMouseCursor true)
          (Class|ChatWindow|SetFocusonInput (Variables|/Script/GamedevNosatov3dP.MyHUD|GetChatWindow _asbp_hud)))))))

(fn ConstructionScript)

(fn AddWeapon
  (params (WeaponIcon :type Texture%202D%20Object%20Reference))
  (bind _aswbp_carousel_click (Utilities|Casting|CastToWBP_CarouselClick (Variables|Default|GetWidgetSwitchMenu)))
  (Default|AddWeapon _aswbp_carousel_click WeaponIcon))