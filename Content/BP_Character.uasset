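; Character Blueprint that exercises saving and loading, with debug prints to check a WeaponRange value.
; Releasing the SaveGame input sets WeaponRange to a fixed value, then calls Save using the player's BP_PlayerController.
; BeginPlay calls Load through the same controller cast and prints WeaponRange, while EndPlay prints a debug message.
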(event EventBeginPlay
  (bind _asbp_player_controller (Utilities|Casting|CastToBP_PlayerController (Game|GetPlayerController 0)))
  (Class|GamedevNosatov3dPCharacter|Load _asbp_player_controller)
  (Development|PrintString (Utilities|String|ToString(Float) (Variables|Default|GetWeaponRange)) true true "(R=0.000000,G=0.660000,B=1.000000,A=1.000000)" 5.0))

(event Collision|EventActorBeginOverlap
  (params (OtherActor :type Actor%20Object%20Reference)))

(event EventTick
  (params (DeltaSeconds :type Float%20%28single-precision%29)))

(event EventEndPlay
  (params (EndPlayReason :type EEndPlayReason%20Enum :default "Destroyed"))
  (Development|PrintString "Char End Play!!!"))

(event Input|ActionEvents|InputActionSaveGame
  (params (Key :type Key%20Structure :default "None"))
  (:Released
    (Variables|Default|SetWeaponRange 3e+03)
    (bind _asbp_player_controller (Utilities|Casting|CastToBP_PlayerController (Game|GetPlayerController 0)))
    (Class|GamedevNosatov3dPCharacter|Save _asbp_player_controller)))

(fn ConstructionScript)