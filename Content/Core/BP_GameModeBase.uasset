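; BP_GameModeBase is a game mode Blueprint that prints debug messages for its Init and UpdateInfo events.
; UpdateInfo prints the display name of CurrentSpawnActor, labelled as a BlueprintImplementableEvent, and Init prints a fixed message.
; BeginPlay, Tick and the construction script are empty.
; A SpawnUnit call on CurrentSpawnActor, followed by a name print, is left unconnected and never runs.
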(event EventBeginPlay
  ;[1 1 1] Begin play
)

(event EventTick
  (params (DeltaSeconds :type Float%20%28single-precision%29)))

(event EventUpdateInfo
  ;[1 1 1] Update Unit Info
  (Development|PrintString (Utilities|String|Append (Utilities|String|MakeLiteralString "BlueprintImplementableEvent. Current spawn Actor = ") (Utilities|GetDisplayName (Variables|Default|GetCurrentSpawnActor)))))

(event EventInit
  ;[1 1 1] Init
  (Development|PrintString "Init Blueprint"))

(fn ConstructionScript)